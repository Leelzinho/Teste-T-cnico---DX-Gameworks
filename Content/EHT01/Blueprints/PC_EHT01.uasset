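; PC_EHT01 is a player controller that maps axis inputs to pawn movement and camera look.
; Move Forward and Move Right add movement input to the controlled pawn along its actor forward and right vectors.
; Turn Right and Look Up apply raw yaw and pitch input, while their Rate variants scale by TurnRateGamepad and world delta seconds for frame-rate-independent turning.
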(event `InputAxis|Turn Right Rate`
  (params (AxisValue :type "Float (single-precision)"))
  ;[1 1 1] Camera
  (`self.AddYawInput` (* AxisValue (`self.Turn Rate Gamepad`) (`GameplayStatics.GetWorldDeltaSeconds`))))

(event `InputAxis|Move Forward`
  (params (AxisValue :type "Float (single-precision)"))
  (bind _returnvalue (`self.K2_GetPawn`))
  ;[1 1 1] Movement
  (`Pawn.AddMovementInput` _returnvalue (`self.GetActorForwardVector` _returnvalue) AxisValue false))

(event `InputAxis|Move Right`
  (params (AxisValue :type "Float (single-precision)"))
  (bind _returnvalue (`self.K2_GetPawn`))
  ;[1 1 1] Movement
  (`Pawn.AddMovementInput` _returnvalue (`self.GetActorRightVector` _returnvalue) AxisValue false))

(event `InputAxis|Look Up Rate`
  (params (AxisValue :type "Float (single-precision)"))
  ;[1 1 1] Camera
  (`self.AddPitchInput` (* AxisValue (`self.Turn Rate Gamepad`) (`GameplayStatics.GetWorldDeltaSeconds`))))

(event `InputAxis|Turn Right`
  (params (AxisValue :type "Float (single-precision)"))
  ;[1 1 1] Camera
  (`self.AddYawInput` AxisValue))

(event `InputAxis|Look Up`
  (params (AxisValue :type "Float (single-precision)"))
  ;[1 1 1] Camera
  (`self.AddPitchInput` AxisValue))

(fn `UserConstructionScript`)