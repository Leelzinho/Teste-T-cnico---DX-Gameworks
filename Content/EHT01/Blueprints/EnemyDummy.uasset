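; Enemy dummy pawn that patrols, shoots at the player, and takes damage from projectiles.
; Tick drives AIMoveTo back and forth along a Movement vector with random pauses, randomizes material color when flagged, and destroys it at zero health.
; Pawn sensing triggers BP_Projectile shots from the Sphere's location, capped by a never-reset MaxShoot counter.
; Projectile hits add score, deal damage with a yaw-based bonus, then briefly stun movement.
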(event `self.ReceiveTick`
  (params (DeltaSeconds :type "Float (single-precision)"))
  (bind _returnvalue (`KismetMathLibrary.RandomFloatInRange` 0.0 5.0))
  (bind _movement (`self.Movement`))
  (bind _floatingpawnmovement (`self.FloatingPawnMovement`))
  (bind _returnvalue_2 (`KismetMathLibrary.NegateVector` _movement))
  (`|ExecutionSequence`
    (:`then_0`
      ;[1 1 1] EnemyDummy Movement
      (if (and (`self.Direction`) (`self.IsMoving`))
        (`|AIMoveTo` self _movement self 3.0
          (:`then`
            _)
          (:`OnSuccess`
            (`self.AddMovementInput` self _movement 1.0 false)))
        (`KismetSystemLibrary.Delay` _returnvalue)
        (set `self.Direction` false)
        (else
          (`|AIMoveTo` self _returnvalue_2 self 3.0
            (:`OnSuccess`
              (`self.AddMovementInput` self _returnvalue_2 1.0 false)
              (`KismetSystemLibrary.Delay` _returnvalue)
              (set `self.Direction` true))))))
    (:`then_1`
      ;[1 1 1] Projectile Spawn Logic
      (while (and (`self.CanSee`) (< (`self.ShootRate`) (`self.MaxShoot`)))
        (cast `/Game/EHT01/Blueprints/BP_FirstPersonCharacter` (stale `self.AIPawnSensing.OnSeePawn` Pawn))
        (`|SpawnActorFromClass` "/Game/EHT01/Blueprints/BP_Projectile.BP_Projectile_C" (`KismetMathLibrary.MakeTransform` (`SceneComponent.K2_GetComponentLocation` (`self.Sphere`)) (`SceneComponent.GetSocketRotation` (`self.EnemyDummy_Mesh`) "Ammo")) "Undefined" "OverrideRootScale" null null)
        (`GameplayStatics.PlaySoundAtLocation` "/Game/FPWeapon/Audio/FirstPersonTemplateWeaponFire02.FirstPersonTemplateWeaponFire02" (`SceneComponent.GetSocketLocation` (`self.EnemyDummy_Mesh`) "Ammo") (struct) 1.0 1.0 0.0 null null null null)
        (`/Engine/EditorBlueprintResources/StandardMacros.IncrementInt` (`self.ShootRate`)
          (:`  `
            (set `self.CanSee` false)))))
    (:`then_2`
      ;[1 1 1] Destroy player when life is 0
      (if (<= (`self.EnemyHealth`) 0)
        (`self.K2_DestroyActor`)))
    (:`then_3`
      ;[1 1 1] Stun
      (if (`self.IsStun`)
        (set `self.IsMoving` false)
        (`ActorComponent.Deactivate` _floatingpawnmovement)
        (`KismetSystemLibrary.Delay` 5.0)
        (set `self.IsStun` false)
        (else
          (set `self.IsMoving` true)
          (`ActorComponent.Activate` _floatingpawnmovement false))))
    (:`then_4`
      (if (`self.Color`)
        (bind _returnvalue_3 (`PrimitiveComponent.CreateDynamicMaterialInstance` (`self.EnemyDummy_Mesh`) 0 "/Game/EnemyDummy/M_EnemyDummy.M_EnemyDummy" "None"))
        (`MaterialInstanceDynamic.SetVectorParameterValue` _returnvalue_3 "base" (make `LinearColor` (`KismetMathLibrary.RandomFloat`) (`KismetMathLibrary.RandomFloat`) (`KismetMathLibrary.RandomFloat`) 1.0))
        (set `self.Color` false)))))

(event `self.AIPawnSensing.OnSeePawn`
  (params (Pawn :type "Pawn Object Reference"))
  ;[1 1 1] Enemy Sees Player
  (set `self.CanSee` true))

(event `self.ReceiveHit`
  (params (MyComp :type "PrimitiveComponent Object Reference") (Other :type "Actor Object Reference") (OtherComp :type "PrimitiveComponent Object Reference") (bSelfMoved :type Boolean) (HitLocation :type "Vector Structure") (HitNormal :type "Vector Structure") (NormalImpulse :type "Vector Structure") (Hit :type "HitResult Structure (by ref)"))
  (bind (_returnvalue_roll _returnvalue_pitch _returnvalue_yaw) (`KismetMathLibrary.BreakRotator` (`KismetMathLibrary.FindLookAtRotation` HitLocation (`self.K2_GetActorLocation` (`GameplayStatics.GetPlayerCharacter` 0)))))
  ;[1 1 1] Receive Damage
  (bind _asbp_projectile (cast `/Game/EHT01/Blueprints/BP_Projectile` Other))
  (set `self.Score` (+ (`self.Score`) 10))
  (if (>= _returnvalue_yaw 0.0)
    (set `self.EnemyHealth` (- (`self.EnemyHealth`) (`/Game/EHT01/Blueprints/BP_Projectile.PlayerDamage` _asbp_projectile)))
    (`KismetSystemLibrary.Delay` 1.0)
    (set `self.IsStun` true)
    (else
      (set `self.EnemyHealth` (- (`self.EnemyHealth`) (+ (`/Game/EHT01/Blueprints/BP_Projectile.PlayerDamage` _asbp_projectile) (`self.ExtraDamage`))))
      (`KismetSystemLibrary.Delay` 1.0)
      (set `self.ExtraDamage` 2)
      (set `self.IsStun` true))))

(fn `UserConstructionScript`)